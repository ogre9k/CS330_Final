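; BP_PForkProjectile is a player bullet spawner that turns one shot into a three-way fork.
; On BeginPlay it spawns three BP_PAirShot actors at its own location: one along its rotation and two yawed 15 degrees to either side.
; It then destroys itself immediately, so all further projectile behavior is left to the spawned shots.
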(event `self.ReceiveBeginPlay`
  (bind _returnvalue (`self.K2_GetActorLocation`))
  (`|SpawnActorFromClass` "/Game/Blueprints/Bullets/PlayerBullets/BP_PAirShot.BP_PAirShot_C" (`KismetMathLibrary.MakeTransform` _returnvalue (`self.K2_GetActorRotation`)) "AlwaysSpawn" "OverrideRootScale" null null)
  (`|SpawnActorFromClass` "/Game/Blueprints/Bullets/PlayerBullets/BP_PAirShot.BP_PAirShot_C" (`KismetMathLibrary.MakeTransform` _returnvalue (`KismetMathLibrary.MakeRotator` (.roll (`self.K2_GetActorRotation`)) (.pitch (`self.K2_GetActorRotation`)) (+ (.yaw (`self.K2_GetActorRotation`)) 15.0))) "AlwaysSpawn" "OverrideRootScale" null null)
  (`|SpawnActorFromClass` "/Game/Blueprints/Bullets/PlayerBullets/BP_PAirShot.BP_PAirShot_C" (`KismetMathLibrary.MakeTransform` _returnvalue (`KismetMathLibrary.MakeRotator` (.roll (`self.K2_GetActorRotation`)) (.pitch (`self.K2_GetActorRotation`)) (+ (.yaw (`self.K2_GetActorRotation`)) -15.0))) "AlwaysSpawn" "OverrideRootScale" null null)
  (`self.K2_DestroyActor`))

(fn `UserConstructionScript`)