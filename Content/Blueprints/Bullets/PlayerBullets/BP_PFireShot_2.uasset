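; BP_PFireShot_2 is a player bullet, a fire shot that changes course in flight at regular intervals.
; A looping timer started on BeginPlay flips the sign of ZigOffset and adds it to the Y component of the ProjectileMovement velocity.
; Because the offsets accumulate, Y velocity alternates between its initial value and a positive-shifted one, giving a stepped drift along world Y rather than a centred zigzag.
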(event `self.ReceiveBeginPlay`
  (set `self.ZigOffset` -1000.0)
  (`KismetSystemLibrary.K2_SetTimerDelegate` (delegate `Reverse`) 0.2 true))

(event `Reverse`
  (bind _projectilemovement (`self.ProjectileMovement`))
  (set `self.ZigOffset` (* (`self.ZigOffset`) -1.0))
  (set `MovementComponent.Velocity` (`KismetMathLibrary.MakeVector` (.x (`MovementComponent.Velocity` _projectilemovement)) (+ (.y (`MovementComponent.Velocity` _projectilemovement)) (`self.ZigOffset`)) (.z (`MovementComponent.Velocity` _projectilemovement))) _projectilemovement))

(fn `UserConstructionScript`)