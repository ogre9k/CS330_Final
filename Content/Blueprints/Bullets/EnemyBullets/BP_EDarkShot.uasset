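; BP_EDarkShot is an enemy bullet projectile that freezes in place while time is stopped.
; On BeginPlay it caches the CS330_FinalGameMode and the projectile movement's starting velocity.
; Its StopTime event reads the game mode's TimeStopped flag, zeroing the velocity when set and restoring the cached velocity otherwise.
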(event `self.ReceiveBeginPlay`
  (bind _ascs330_final_game_mode (cast `CS330_FinalGameMode` (`GameplayStatics.GetGameMode`)))
  (set `self.MyGameMode` _ascs330_final_game_mode)
  (set `self.InitialVelocity` (`MovementComponent.Velocity` (`self.ProjectileMovement`))))

(event `self.ReceiveTick`
  (params (DeltaSeconds :type "Float (single-precision)")))

(event `StopTime`
  (if (`CS330_FinalGameMode.TimeStopped` (`self.MyGameMode`))
    (set `MovementComponent.Velocity` (0.0 0.0 0.0) (`self.ProjectileMovement`))
    (else
      (set `MovementComponent.Velocity` (`self.InitialVelocity`) (`self.ProjectileMovement`)))))

(fn `UserConstructionScript`)