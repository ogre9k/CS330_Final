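; Enemy bullet spawner in the Patchouli bullet set that fires rings of blue helper bullets.
; On BeginPlay it calls SpawnStuff four times in quick succession, separated by short delays.
; Each call loops ShootBullet to launch BP_E20Circle_HelperBlue from Center at evenly stepped angles around a full circle.
; The inclusive loop makes 21 shots, so the last overlaps the first direction.
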(event `self.ReceiveBeginPlay`
  (`parent.ReceiveBeginPlay`)
  (`KismetSystemLibrary.Delay` 0.1)
  (`self.SpawnStuff`)
  (`KismetSystemLibrary.Delay` 0.1)
  (`self.SpawnStuff`)
  (`KismetSystemLibrary.Delay` 0.1)
  (`self.SpawnStuff`)
  (`KismetSystemLibrary.Delay` 0.1)
  (`self.SpawnStuff`))

(fn `SpawnStuff`
  (for _index (range 21)
    (`self.Shoot Bullet` "/Game/Blueprints/Bullets/EnemyBullets/Patchouli/20Circle/BP_E20Circle_HelperBlue.BP_E20Circle_HelperBlue_C" (`self.Center`) (`KismetMathLibrary.Conv_IntToDouble` (* _index 18)))))

(fn `UserConstructionScript`
  (`parent.UserConstructionScript`))