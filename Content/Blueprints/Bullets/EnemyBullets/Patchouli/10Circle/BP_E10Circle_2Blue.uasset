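; Enemy bullet pattern Blueprint in the Patchouli 10Circle set that fires three timed waves of player-aimed bullets when spawned.
; BeginPlay runs SetLocations, then plays a laser sound before each wave, with short delays between them.
; SetLocations derives numbered spawn points from actor-relative Front, Back, Left and Right markers plus fixed offsets.
; The first two waves fire four shots each and the third seven, all via ShootBullet using the first Bullets entry.
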(event `self.ReceiveBeginPlay`
  (bind _output (`|GetArrayItem` (`self.Bullets`)))
  (`parent.ReceiveBeginPlay`)
  (`self.SetLocations`)
  (`KismetSystemLibrary.Delay` 0.1)
  (`GameplayStatics.PlaySound2D` "/Game/OurAudio/test/NFF-laser.NFF-laser" 1.0 1.0 0.0 null null)
  (`self.FirstWave` _output)
  (`KismetSystemLibrary.Delay` 0.7)
  (`GameplayStatics.PlaySound2D` "/Game/OurAudio/test/NFF-laser.NFF-laser" 1.0 1.0 0.0 null null)
  (`self.SecondWave` _output)
  (`KismetSystemLibrary.Delay` 0.7)
  (`GameplayStatics.PlaySound2D` "/Game/OurAudio/test/NFF-laser.NFF-laser" 1.0 1.0 0.0 null null)
  (`self.ThirdWave` _output))

(fn `FirstWave`
  (params (Bullet :type "EnemyProjectile Class Reference"))
  (`self.Shoot Bullet` Bullet (`self.1`) 0.0 true)
  (`self.Shoot Bullet` Bullet (`self.2`) 0.0 true)
  (`self.Shoot Bullet` Bullet (`self.3`) (`KismetMathLibrary.Conv_IntToDouble` (* 0 36)) true)
  (`self.Shoot Bullet` Bullet (`self.4`) 0.0 true))

(fn `SecondWave`
  (params (Bullet :type "EnemyProjectile Class Reference"))
  (`self.Shoot Bullet` Bullet (`self.5`) 0.0 true)
  (`self.Shoot Bullet` Bullet (`self.6`) 0.0 true)
  (`self.Shoot Bullet` Bullet (`self.7`) 0.0 true)
  (`self.Shoot Bullet` Bullet (`self.8`) 0.0 true))

(fn `SetLocations`
  (bind _returnvalue (`self.K2_GetActorLocation`))
  (bind _returnvalue_2 (`self.K2_GetActorLocation`))
  (bind _returnvalue_3 (`self.K2_GetActorLocation`))
  (bind _returnvalue_4 (`self.K2_GetActorLocation`))
  (set `self.1` (+ (+ (+ (- (`self.Front`) _returnvalue_3) (- _returnvalue_3 (`self.Left`))) (`self.K2_GetActorLocation`)) (-150.0 -200.0 0.0)))
  (set `self.2` (+ (+ (+ (- (`self.Front`) _returnvalue_2) (- _returnvalue_2 (`self.Right`))) (`self.K2_GetActorLocation`)) (-150.0 200.0 0.0)))
  (set `self.3` (+ (+ (+ (- (`self.Back`) _returnvalue_4) (- _returnvalue_4 (`self.Left`))) (`self.K2_GetActorLocation`)) (150.0 -200.0 0.0)))
  (set `self.4` (+ (+ (+ (- (`self.Back`) _returnvalue) (- _returnvalue (`self.Right`))) (`self.K2_GetActorLocation`)) (150.0 200.0 0.0)))
  (set `self.5` (+ (`self.1`) (100.0 -100.0 0.0)))
  (set `self.6` (+ (`self.2`) (100.0 100.0 0.0)))
  (set `self.7` (+ (`self.3`) (100.0 100.0 0.0)))
  (set `self.8` (+ (`self.4`) (-100.0 100.0 0.0)))
  (set `self.9` (+ (`self.2`) (-100.0 0.0 0.0)))
  (set `self.10` (+ (`self.1`) (100.0 0.0 0.0)))
  (set `self.11` (`self.5`))
  (set `self.12` (`self.6`))
  (set `self.13` (`self.Center`))
  (set `self.14` (+ (`self.3`) (0.0 -100.0 0.0)))
  (set `self.15` (+ (`self.4`) (0.0 -100.0 0.0))))

(fn `ThirdWave`
  (params (Bullet :type "EnemyProjectile Class Reference"))
  (`self.Shoot Bullet` Bullet (`self.9`) 0.0 true)
  (`self.Shoot Bullet` Bullet (`self.10`) 0.0 true)
  (`self.Shoot Bullet` Bullet (`self.11`) 0.0 true)
  (`self.Shoot Bullet` Bullet (`self.12`) 0.0 true)
  (`self.Shoot Bullet` Bullet (`self.13`) 0.0 true)
  (`self.Shoot Bullet` Bullet (`self.14`) 0.0 true)
  (`self.Shoot Bullet` Bullet (`self.15`) 0.0 true))

(fn `UserConstructionScript`
  (`parent.UserConstructionScript`))