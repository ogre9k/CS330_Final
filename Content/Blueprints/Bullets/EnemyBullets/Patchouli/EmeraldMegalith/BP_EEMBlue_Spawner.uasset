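; Enemy bullet spawner for the blue part of Patchouli's Emerald Megalith pattern.
; On BeginPlay it picks one of three bullet types at random and scatters a burst around Center with random offsets and directions.
; It also defines three wave functions that fire radial rings from points computed in SetLocations relative to the arena markers, though this graph calls none of them.
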(event `self.ReceiveBeginPlay`
  (`parent.ReceiveBeginPlay`)
  (set `self.RandomInt` (`KismetMathLibrary.RandomInteger` 3))
  (for _ (range 17)
    (`self.Shoot Bullet` (`|GetArrayItem` (`self.Bullets`) (`self.RandomInt`)) (`KismetMathLibrary.MakeVector` (+ (.x (`self.Center`)) (`KismetMathLibrary.RandomFloatInRange` -100.0 100.0)) (+ (.y (`self.Center`)) (`KismetMathLibrary.RandomFloatInRange` -100.0 100.0)) (.z (`self.Center`))) (* (`KismetMathLibrary.RandomFloat`) 360.0))))

(fn `FirstWave`
  (params (Bullet :type "EnemyProjectile Class Reference"))
  (for _index (range 11)
    (`self.Shoot Bullet` Bullet (`self.1`) (`KismetMathLibrary.Conv_IntToDouble` (* _index 36))))
  (for _index_2 (range 11)
    (`self.Shoot Bullet` Bullet (`self.2`) (`KismetMathLibrary.Conv_IntToDouble` (* _index_2 36))))
  (for _index_3 (range 11)
    (`self.Shoot Bullet` Bullet (`self.3`) (`KismetMathLibrary.Conv_IntToDouble` (* _index_3 36))))
  (for _index_4 (range 11)
    (`self.Shoot Bullet` Bullet (`self.4`) (`KismetMathLibrary.Conv_IntToDouble` (* _index_4 36)))))

(fn `SecondWave`
  (params (Bullet :type "EnemyProjectile Class Reference"))
  (for _index (range 11)
    (`self.Shoot Bullet` Bullet (`self.5`) (`KismetMathLibrary.Conv_IntToDouble` (* _index 36))))
  (for _index_2 (range 11)
    (`self.Shoot Bullet` Bullet (`self.6`) (`KismetMathLibrary.Conv_IntToDouble` (* _index_2 36))))
  (for _index_3 (range 11)
    (`self.Shoot Bullet` Bullet (`self.7`) (`KismetMathLibrary.Conv_IntToDouble` (* _index_3 36))))
  (for _index_4 (range 11)
    (`self.Shoot Bullet` Bullet (`self.8`) (`KismetMathLibrary.Conv_IntToDouble` (* _index_4 36)))))

(fn `SetLocations`
  (bind _returnvalue (`self.K2_GetActorLocation`))
  (bind _returnvalue_2 (`self.K2_GetActorLocation`))
  (bind _returnvalue_3 (`self.K2_GetActorLocation`))
  (bind _returnvalue_4 (`self.K2_GetActorLocation`))
  (set `self.1` (+ (+ (+ (- (`self.Front`) _returnvalue_3) (- _returnvalue_3 (`self.Left`))) (`self.K2_GetActorLocation`)) (-150.0 -200.0 0.0)))
  (set `self.2` (+ (+ (+ (- (`self.Front`) _returnvalue_2) (- _returnvalue_2 (`self.Right`))) (`self.K2_GetActorLocation`)) (-150.0 200.0 0.0)))
  (set `self.3` (+ (+ (+ (- (`self.Back`) _returnvalue_4) (- _returnvalue_4 (`self.Left`))) (`self.K2_GetActorLocation`)) (150.0 -200.0 0.0)))
  (set `self.4` (+ (+ (+ (- (`self.Back`) _returnvalue) (- _returnvalue (`self.Right`))) (`self.K2_GetActorLocation`)) (150.0 200.0 0.0)))
  (set `self.5` (+ (`self.1`) (100.0 -100.0 0.0)))
  (set `self.6` (+ (`self.2`) (100.0 100.0 0.0)))
  (set `self.7` (+ (`self.3`) (100.0 100.0 0.0)))
  (set `self.8` (+ (`self.4`) (-100.0 100.0 0.0)))
  (set `self.9` (+ (`self.2`) (-100.0 0.0 0.0)))
  (set `self.10` (+ (`self.1`) (100.0 0.0 0.0)))
  (set `self.11` (`self.5`))
  (set `self.12` (`self.6`))
  (set `self.13` (`self.Center`))
  (set `self.14` (+ (`self.3`) (0.0 -100.0 0.0)))
  (set `self.15` (+ (`self.4`) (0.0 -100.0 0.0))))

(fn `ThirdWave`
  (params (Bullet :type "EnemyProjectile Class Reference"))
  (for _index (range 11)
    (`self.Shoot Bullet` Bullet (`self.9`) (`KismetMathLibrary.Conv_IntToDouble` (* _index 36))))
  (for _index_2 (range 11)
    (`self.Shoot Bullet` Bullet (`self.10`) (`KismetMathLibrary.Conv_IntToDouble` (* _index_2 36))))
  (for _index_3 (range 11)
    (`self.Shoot Bullet` Bullet (`self.11`) (`KismetMathLibrary.Conv_IntToDouble` (* _index_3 36))))
  (for _index_4 (range 11)
    (`self.Shoot Bullet` Bullet (`self.12`) (`KismetMathLibrary.Conv_IntToDouble` (* _index_4 36))))
  (for _index_5 (range 11)
    (`self.Shoot Bullet` Bullet (`self.13`) (`KismetMathLibrary.Conv_IntToDouble` (* _index_5 36))))
  (for _index_6 (range 11)
    (`self.Shoot Bullet` Bullet (`self.14`) (`KismetMathLibrary.Conv_IntToDouble` (* _index_6 36))))
  (for _index_7 (range 11)
    (`self.Shoot Bullet` Bullet (`self.15`) (`KismetMathLibrary.Conv_IntToDouble` (* _index_7 36)))))

(fn `UserConstructionScript`
  (`parent.UserConstructionScript`))