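; Blue enemy bullet for Patchouli's Rage Trilithon attack that changes speed in phases before scattering.
; On BeginPlay, the Slowdown timeline scales the initial velocity at a random play rate, so each bullet's timing differs.
; A second timeline then scales that velocity again.
; After a short delay, the bullet takes a random velocity in the XY plane, with Z zeroed.
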(event `self.ReceiveBeginPlay`
  (`parent.ReceiveBeginPlay`)
  (`TimelineComponent.SetPlayRate` (`self.Slowdown`) (`KismetMathLibrary.RandomFloatInRange` 0.5 2.0))
  (bind (_direction _speedpercentage) (`Timeline|Slowdown`)
    (:`Update`
      (set `MovementComponent.Velocity` (* (`self.InitialVelocity`) _speedpercentage) (`self.ProjectileMovement`)))
    (:`Finished`
      (bind (_direction_2 _speedpercentage_2) (`Timeline|Timeline_0`)
        (:`Update`
          (set `MovementComponent.Velocity` (* (`self.InitialVelocity`) _speedpercentage_2) (`self.ProjectileMovement`)))
        (:`Finished`
          (`KismetSystemLibrary.Delay` 0.3)
          (set `MovementComponent.Velocity` (* (`KismetMathLibrary.MakeVector` (.x (`KismetMathLibrary.RandomUnitVector`)) (.y (`KismetMathLibrary.RandomUnitVector`))) 900.0) (`self.ProjectileMovement`)))))))

(fn `UserConstructionScript`
  (`parent.UserConstructionScript`))