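; BP_ExampleEmitter is an example bullet-pattern emitter that starts firing on BeginPlay and changes its shot pattern across five phases.
; Each FireShot event checks the current phase and calls that phase's function, which shoots colored orb bullets from the center at fixed directions, from four-way crosses down to single shots.
; Tick rotates the emitter during the first and last phases, so those shots sweep around over time.
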(event `self.FireShot`
  ;[1 1 1] Check phase and shoot appropriate bullet
  (bind _result (`self.IsPhase` 0))
  (if _result
    (`self.Phase1Shoot`)
    (else
      (bind _result_2 (`self.IsPhase` 1))
      (if _result_2
        (`self.Phase2Shoot`)
        (else
          (bind _result_3 (`self.IsPhase` 2))
          (if _result_3
            (`self.Phase3Shoot`)
            (else
              (bind _result_4 (`self.IsPhase` 3))
              (if _result_4
                (`self.Phase4Shoot`)
                (else
                  (bind _result_5 (`self.IsPhase` 4))
                  (if _result_5
                    (`self.Phase5Shoot`)))))))))))

(event `self.ReceiveBeginPlay`
  ;[1 1 1] Start shooting immediately
  (`self.StartFire`))

(event `self.ReceiveTick`
  (params (DeltaSeconds :type "Float (single-precision)"))
  ;[1 1 1] Constantly rotate during phases 1 and 5
  (bind _result (`self.IsPhase` 0))
  (bind _result_2 (`self.IsPhase` 4))
  (if (or _result _result_2)
    (`self.Rotate` 1.0)))

(fn `Phase1Shoot`
  (`self.Shoot Bullet` "/Game/Blueprints/Bullets/EnemyBullets/BP_EBlueOrb.BP_EBlueOrb_C" (`self.Center`))
  (`self.Shoot Bullet` "/Game/Blueprints/Bullets/EnemyBullets/BP_EBlueOrb.BP_EBlueOrb_C" (`self.Center`) 90.0)
  (`self.Shoot Bullet` "/Game/Blueprints/Bullets/EnemyBullets/BP_EBlueOrb.BP_EBlueOrb_C" (`self.Center`) 180.0)
  (`self.Shoot Bullet` "/Game/Blueprints/Bullets/EnemyBullets/BP_EBlueOrb.BP_EBlueOrb_C" (`self.Center`) 270.0))

(fn `Phase2Shoot`
  (`self.Shoot Bullet` "/Game/Blueprints/Bullets/EnemyBullets/BP_EBlueOrb.BP_EBlueOrb_C" (`self.Center`) 45.0)
  (`self.Shoot Bullet` "/Game/Blueprints/Bullets/EnemyBullets/BP_ERedOrb.BP_ERedOrb_C" (`self.Center`) 225.0)
  (`self.Shoot Bullet` "/Game/Blueprints/Bullets/EnemyBullets/BP_EGreenOrb.BP_EGreenOrb_C" (`self.Center`) 135.0)
  (`self.Shoot Bullet` "/Game/Blueprints/Bullets/EnemyBullets/BP_EBlueOrb.BP_EBlueOrb_C" (`self.Center`) 315.0))

(fn `Phase3Shoot`
  (`self.Shoot Bullet` "/Game/Blueprints/Bullets/EnemyBullets/BP_EGreenOrb.BP_EGreenOrb_C" (`self.Center`))
  (`self.Shoot Bullet` "/Game/Blueprints/Bullets/EnemyBullets/BP_EGreenOrb.BP_EGreenOrb_C" (`self.Center`) 90.0)
  (`self.Shoot Bullet` "/Game/Blueprints/Bullets/EnemyBullets/BP_EGreenOrb.BP_EGreenOrb_C" (`self.Center`) 180.0)
  (`self.Shoot Bullet` "/Game/Blueprints/Bullets/EnemyBullets/BP_EGreenOrb.BP_EGreenOrb_C" (`self.Center`) 270.0))

(fn `Phase4Shoot`
  (`self.Shoot Bullet` "/Game/Blueprints/Bullets/EnemyBullets/BP_ERedOrb.BP_ERedOrb_C" (`self.Center`) 180.0))

(fn `Phase5Shoot`
  (`self.Shoot Bullet` "/Game/Blueprints/Bullets/EnemyBullets/BP_EBlueOrb.BP_EBlueOrb_C" (`self.Center`)))

(fn `UserConstructionScript`
  (`parent.UserConstructionScript`))