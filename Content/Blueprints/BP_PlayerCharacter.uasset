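; Player character Blueprint that casts fire, water and air spell cards, switching bullet type and cast effect to match the element.
; Card inputs call the DeckHandler found at BeginPlay; the UseCard event maps CardToUse to an element, clears prior effects and spawns it, wrapping some shots in aim setup.
; Number keys provide a parallel hard-coded cast path by CardIndex tier, cycled through debug SwapCards.
; StopTime toggles the GameMode flag and notifies enemy dark shots.
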(event `InputAction|FirstCard`
  (params (Key :type "Key Structure"))
  (:`Pressed`
    (`DeckHandler.UseCard` (`self.MyDeck`) 0)))

(event `self.UseCard`
  (`self.ShootUsedCard`))

(event `InputAction|SecondCard`
  (params (Key :type "Key Structure"))
  (:`Pressed`
    (`DeckHandler.UseCard` (`self.MyDeck`) 1)))

(event `InputAction|ThirdCard`
  (params (Key :type "Key Structure"))
  (:`Pressed`
    (`DeckHandler.UseCard` (`self.MyDeck`) 2)))

(event `InputAction|SwapCards`
  (params (Key :type "Key Structure"))
  ;[1 1 1] DEBUG - Disable before release
  (:`Pressed`
    (`self.SwapCardSet`)))

(event `self.ReceiveBeginPlay`
  (`self.FindDeck`))

(event `InputAction|OneKey`
  (params (Key :type "Key Structure"))
  ;[1 1 1] DEBUG - Disable before release
  (:`Pressed`
    (`self.UseFireCard`)))

(event `InputAction|TwoKey`
  (params (Key :type "Key Structure"))
  ;[1 1 1] DEBUG - Disable before release
  (:`Pressed`
    (`self.UseWaterCard`)))

(event `InputAction|ThreeKey`
  (params (Key :type "Key Structure"))
  ;[1 1 1] DEBUG - Disable before release
  (:`Pressed`
    (`self.UseAirCard`)))

(fn `AfterShootCard`
  (params (ShootingOrNot :type Boolean))
  (if (not ShootingOrNot)
    (set `self.Shooting` false)))

(fn `BeforeShootCard`
  (returns (ShootOrNot :type Boolean))
  (`self.UpdateMouseLook`)
  (set `self.SpawnTransform` (`KismetMathLibrary.MakeTransform` (`self.K2_GetActorLocation`) (`self.K2_GetActorRotation`)))
  (if (`self.Shooting`)
    (return true)
    (else
      (set `self.Shooting` true)
      (set `self.LastRotation` (`self.K2_GetActorRotation`))
      (return false))))

(fn `CleanUp`
  (`ActorComponent.Deactivate` (`self.BlueCast`))
  (`ActorComponent.Deactivate` (`self.GreenCast`))
  (`ActorComponent.Deactivate` (`self.RedCast`))
  ;[1 1 1] Set firing rate back to default
  (if (`self.Shooting`)
    (`self.OnStopFire`)
    (set `self.FireRate` 0.16)
    (`self.OnStartFire`)
    (bind _outactors (`GameplayStatics.GetAllActorsOfClass` "/Game/Blueprints/Cards/Buffs/BP_CDeluge.BP_CDeluge_C"))
    (for _array_element _outactors
      (`self.K2_DestroyActor` _array_element))
    (bind _outactors_2 (`GameplayStatics.GetAllActorsOfClass` "/Game/Blueprints/Cards/Buffs/BP_COverheat.BP_COverheat_C"))
    (for _array_element_2 _outactors_2
      (`self.K2_DestroyActor` _array_element_2))
    (bind _outactors_3 (`GameplayStatics.GetAllActorsOfClass` "/Game/Blueprints/Cards/Buffs/BP_CBlitz.BP_CBlitz_C"))
    (for _array_element_3 _outactors_3
      (`self.K2_DestroyActor` _array_element_3))
    (else
      (set `self.FireRate` 0.16))))

(fn `FindDeck`
  (bind _outactors (`GameplayStatics.GetAllActorsOfClass` "/Script/CS330_Final.DeckHandler"))
  (for _array_element _outactors
    (set `self.MyDeck` _array_element)))

(fn `GetCardInfo`
  (if true
    _))

(fn `ShootUsedCard`
  (bind _tempcolor (`self.tempColor`))
  ;[1 1 1] Figure out which card we're trying to use and set up temp variables for it
  (if (== (`self.CardToUse`) "/Game/Blueprints/Cards/Cantrips/BP_CEmber.BP_CEmber_C")
    (set `self.tempColor` "Red" :!label _label)
    ;[1 1 1] Set spawn transform
    (set `self.SpawnTransform` (`KismetMathLibrary.MakeTransform` (`self.K2_GetActorLocation`) (`self.K2_GetActorRotation`)) :!label _label_2)
    (`self.CleanUp`)
    ;[1 1 1] Check color and set bullet and color graphic
    (if (`KismetStringLibrary.EqualEqual_StrStr` _tempcolor "Red")
      (set `self.Bullet` "/Game/Blueprints/Bullets/PlayerBullets/BP_PFireShot.BP_PFireShot_C")
      (`ActorComponent.Activate` (`self.RedCast`) false)
      (set `self.Color` (`self.tempColor`) :!label _label_3)
      ;[1 1 1] Check if the card is a shot type card, then spawn the card effect
      (if (`self.tempShot`)
        (bind _shootornot (`self.BeforeShootCard`))
        (`|SpawnActorFromClass` (`self.CardToUse`) (`self.SpawnTransform`) "Undefined" "OverrideRootScale" null null)
        (`self.AfterShootCard` _shootornot)
        (set `self.tempShot` false)
        (else
          (`|SpawnActorFromClass` (`self.CardToUse`) (`self.SpawnTransform`) "Undefined" "OverrideRootScale" null null)))
      (elif (`KismetStringLibrary.EqualEqual_StrStr` _tempcolor "Blue")
        (set `self.Bullet` "/Game/Blueprints/Bullets/PlayerBullets/BP_PWaterShot.BP_PWaterShot_C")
        (`ActorComponent.Activate` (`self.BlueCast`) false)
        (goto _label_3)
        (elif (`KismetStringLibrary.EqualEqual_StrStr` _tempcolor "Green")
          (set `self.Bullet` "/Game/Blueprints/Bullets/PlayerBullets/BP_PAirShot.BP_PAirShot_C")
          (`ActorComponent.Activate` (`self.GreenCast`) false)
          (goto _label_3))))
    (elif (== (`self.CardToUse`) "/Game/Blueprints/Cards/Attacks/BP_CFireball.BP_CFireball_C")
      (set `self.tempShot` true)
      (goto _label)
      (elif (== (`self.CardToUse`) "/Game/Blueprints/Cards/Buffs/BP_COverheat.BP_COverheat_C")
        (goto _label)
        (elif (== (`self.CardToUse`) "/Game/Blueprints/Cards/Ultimates/BP_CInferno.BP_CInferno_C")
          (goto _label)
          (elif (== (`self.CardToUse`) "/Game/Blueprints/Cards/Cantrips/BP_CDroplet.BP_CDroplet_C")
            (set `self.tempColor` "Blue" :!label _label_4)
            (goto _label_2)
            (elif (== (`self.CardToUse`) "/Game/Blueprints/Cards/Attacks/BP_CBurst.BP_CBurst_C")
              (goto _label_4)
              (elif (== (`self.CardToUse`) "/Game/Blueprints/Cards/Buffs/BP_CDeluge.BP_CDeluge_C")
                (goto _label_4)
                (elif (== (`self.CardToUse`) "/Game/Blueprints/Cards/Ultimates/BP_CFreeze.BP_CFreeze_C")
                  (goto _label_4)
                  (elif (== (`self.CardToUse`) "/Game/Blueprints/Cards/Cantrips/BP_CBreeze.BP_CBreeze_C")
                    (set `self.tempColor` "Green" :!label _label_5)
                    (goto _label_2)
                    (elif (== (`self.CardToUse`) "/Game/Blueprints/Cards/Attacks/BP_CBoomerang.BP_CBoomerang_C")
                      (set `self.tempShot` true)
                      (goto _label_5)
                      (elif (== (`self.CardToUse`) "/Game/Blueprints/Cards/Buffs/BP_CBlitz.BP_CBlitz_C")
                        (goto _label_5)
                        (elif (== (`self.CardToUse`) "/Game/Blueprints/Cards/Ultimates/BP_CTornado.BP_CTornado_C")
                          (goto _label_5))))))))))))))

(fn `StopTime`
  (bind _ascs330_final_game_mode (cast `CS330_FinalGameMode` (`GameplayStatics.GetGameMode`)))
  (if (`CS330_FinalGameMode.TimeStopped` _ascs330_final_game_mode)
    (set `CS330_FinalGameMode.TimeStopped` false _ascs330_final_game_mode)
    (else
      (set `CS330_FinalGameMode.TimeStopped` true _ascs330_final_game_mode)))
  (bind _outactors (`GameplayStatics.GetAllActorsOfClass` "/Game/Blueprints/Bullets/EnemyBullets/BP_EDarkShot.BP_EDarkShot_C"))
  (for _array_element _outactors
    (bind _asbp_edark_shot (cast `/Game/Blueprints/Bullets/EnemyBullets/BP_EDarkShot` _array_element))
    (`/Game/Blueprints/Bullets/EnemyBullets/BP_EDarkShot.StopTime` _asbp_edark_shot)))

(fn `SwapCardSet`
  (if (== (`self.CardIndex`) 3.0)
    (set `self.CardIndex` 0.0)
    (else
      (set `self.CardIndex` (+ (`self.CardIndex`) 1.0))))
  (if (== (`self.CardIndex`) 0.0)
    (`KismetSystemLibrary.PrintString` "Cantrips")
    (elif (== (`self.CardIndex`) 1.0)
      (`KismetSystemLibrary.PrintString` "Attacks")
      (elif (== (`self.CardIndex`) 2.0)
        (`KismetSystemLibrary.PrintString` "Buffs")
        (elif (== (`self.CardIndex`) 3.0)
          (`KismetSystemLibrary.PrintString` "Ultimates"))))))

(fn `UseAirCard`
  (set `self.SpawnTransform` (`KismetMathLibrary.MakeTransform` (`self.K2_GetActorLocation`) (`self.K2_GetActorRotation`)))
  (`self.CleanUp`)
  (set `self.Bullet` "/Game/Blueprints/Bullets/PlayerBullets/BP_PAirShot.BP_PAirShot_C")
  (`ActorComponent.Activate` (`self.GreenCast`) false)
  (if (== (`self.CardIndex`) 0.0)
    (`GameplayStatics.SpawnEmitterAtLocation` "/Game/OurFX/P_ky_windBallHit.P_ky_windBallHit" (`self.K2_GetActorLocation`))
    (elif (== (`self.CardIndex`) 1.0)
      (bind _shootornot (`self.BeforeShootCard`))
      (`|SpawnActorFromClass` "/Game/Blueprints/Cards/Attacks/BP_CBoomerang.BP_CBoomerang_C" (`self.SpawnTransform`) "Undefined" "OverrideRootScale" null null)
      (`self.AfterShootCard` _shootornot)
      (elif (== (`self.CardIndex`) 2.0)
        (`|SpawnActorFromClass` "/Game/Blueprints/Cards/Buffs/BP_CBlitz.BP_CBlitz_C" (`self.SpawnTransform`) "Undefined" "OverrideRootScale" null null)
        (elif (== (`self.CardIndex`) 3.0)
          (`|SpawnActorFromClass` "/Game/Blueprints/Cards/Ultimates/BP_CTornado.BP_CTornado_C" (`self.SpawnTransform`) "Undefined" "OverrideRootScale" null null))))))

(fn `UseFireCard`
  (set `self.SpawnTransform` (`KismetMathLibrary.MakeTransform` (`self.K2_GetActorLocation`) (`self.K2_GetActorRotation`)))
  (`self.CleanUp`)
  (set `self.Bullet` "/Game/Blueprints/Bullets/PlayerBullets/BP_PFireShot.BP_PFireShot_C")
  (`ActorComponent.Activate` (`self.RedCast`) false)
  (if (== (`self.CardIndex`) 0.0)
    (`GameplayStatics.SpawnEmitterAtLocation` "/Game/OurFX/P_ky_fireballHit.P_ky_fireballHit" (`self.K2_GetActorLocation`))
    (elif (== (`self.CardIndex`) 1.0)
      (bind _shootornot (`self.BeforeShootCard`))
      (`|SpawnActorFromClass` "/Game/Blueprints/Cards/Attacks/BP_CFireball.BP_CFireball_C" (`self.SpawnTransform`) "Undefined" "OverrideRootScale" null null)
      (`self.AfterShootCard` _shootornot)
      (elif (== (`self.CardIndex`) 2.0)
        (`|SpawnActorFromClass` "/Game/Blueprints/Cards/Buffs/BP_COverheat.BP_COverheat_C" (`self.SpawnTransform`) "Undefined" "OverrideRootScale" null null)
        (elif (== (`self.CardIndex`) 3.0)
          (bind _shootornot_2 (`self.BeforeShootCard`))
          (`|SpawnActorFromClass` "/Game/Blueprints/Cards/Ultimates/BP_CInferno.BP_CInferno_C" (`self.SpawnTransform`) "Undefined" "OverrideRootScale" null null)
          (`self.AfterShootCard` _shootornot_2))))))

(fn `UserConstructionScript`)

(fn `UseWaterCard`
  (set `self.SpawnTransform` (`KismetMathLibrary.MakeTransform` (`self.K2_GetActorLocation`) (`self.K2_GetActorRotation`)))
  (`self.CleanUp`)
  (set `self.Bullet` "/Game/Blueprints/Bullets/PlayerBullets/BP_PWaterShot.BP_PWaterShot_C")
  (`ActorComponent.Activate` (`self.BlueCast`) false)
  (if (== (`self.CardIndex`) 0.0)
    (`GameplayStatics.SpawnEmitterAtLocation` "/Game/OurFX/P_ky_waterBallHit.P_ky_waterBallHit" (`self.K2_GetActorLocation`))
    (elif (== (`self.CardIndex`) 1.0)
      (`|SpawnActorFromClass` "/Game/Blueprints/Cards/Attacks/BP_CBurst.BP_CBurst_C" (`self.SpawnTransform`) "Undefined" "OverrideRootScale" null null)
      (elif (== (`self.CardIndex`) 2.0)
        (`|SpawnActorFromClass` "/Game/Blueprints/Cards/Buffs/BP_CDeluge.BP_CDeluge_C" (`self.SpawnTransform`) "Undefined" "OverrideRootScale" null null)
        (elif (== (`self.CardIndex`) 3.0)
          (`|SpawnActorFromClass` "/Game/Blueprints/Cards/Ultimates/BP_CFreeze.BP_CFreeze_C" (`self.SpawnTransform`) "Undefined" "OverrideRootScale" null null))))))