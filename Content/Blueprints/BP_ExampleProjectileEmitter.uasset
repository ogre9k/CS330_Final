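; Example projectile emitter actor that starts firing as soon as play begins.
; BeginPlay calls StartFire, and the FireShot event spawns the first class in the Bullets array.
; Each shot spawns at the Right location, using the emitter's rotation with yaw offset a quarter turn.
; The firing cadence is not defined in this graph, and the overlap, tick and construction hooks are empty.
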(event `self.ReceiveBeginPlay`
  (`self.StartFire`))

(event `self.FireShot`
  (`|SpawnActorFromClass` (`|GetArrayItem` (`self.Bullets`)) (`KismetMathLibrary.MakeTransform` (`self.Right`) (`KismetMathLibrary.MakeRotator` (.roll (`self.K2_GetActorRotation`)) (.pitch (`self.K2_GetActorRotation`)) (+ (.yaw (`self.K2_GetActorRotation`)) 90.0))) "Undefined" "OverrideRootScale" null null))

(fn `UserConstructionScript`)