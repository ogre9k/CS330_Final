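; BP_Room0 is a room Blueprint that supplies randomized spawn locations from arrow components placed in it.
; GetSpawnArrowLocation returns the world location of one of six arrows, picked by a random index.
; GetAttachTransform is an empty stub, and the event graph and construction script contain no logic.
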(fn `GetAttachTransform`)

(fn `GetSpawnArrowLocation`
  (returns (RandomSpawnArrow :type "Vector Structure"))
  (return (`|GetArrayItem` (`|MakeArray` (`SceneComponent.K2_GetComponentLocation` (`self.Arrow`)) (`SceneComponent.K2_GetComponentLocation` (`self.Arrow1`)) (`SceneComponent.K2_GetComponentLocation` (`self.Arrow2`)) (`SceneComponent.K2_GetComponentLocation` (`self.Arrow3`)) (`SceneComponent.K2_GetComponentLocation` (`self.Arrow4`)) (`SceneComponent.K2_GetComponentLocation` (`self.Arrow5`))) (`KismetMathLibrary.RandomIntegerInRange` 0 5))))

(fn `UserConstructionScript`)