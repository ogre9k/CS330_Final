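; Parent boss Character for a phase-based projectile-shooting boss fight, providing shared helpers for firing, attack animation and phases.
; ShootBullet spawns bullets toward the player or at a yaw offset, unless the game mode's time stop is active.
; SetFireRate restarts active fire with a fixed or random-range rate, and ShootAnimate alternates two attack montages.
; ChangePhase updates every emitter in the level, advances the boss's phase and destroys it upon reaching the final phase.
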(event `self.ReceiveBeginPlay`
  (bind _ascs330_final_game_mode (cast `CS330_FinalGameMode` (`GameplayStatics.GetGameMode`)))
  (set `self.My Gamemode` _ascs330_final_game_mode)
  (`self.UpdateOffsets`))

(event `self.ChangePhase`
  (`self.HandleNewPhase`))

(fn `HandleNewPhase`
  (returns (`N/A` :type Boolean))
  (bind _currentphase (`self.CurrentPhase`))
  (set `self.bCanBeDamaged` false)
  ;[1 1 1] Update the phase of each emitter
  (bind _outactors (`GameplayStatics.GetAllActorsOfClass` "/Game/Blueprints/BP_ParentEmitter.BP_ParentEmitter_C"))
  (for _array_element _outactors
    (`/Game/Blueprints/BP_ParentEmitter.UpdatePhase` _array_element))
  ;[1 1 1] Update the phase of the boss and kill it if it's out of phases
  (set `self.CurrentPhase` (+ _currentphase 1))
  (if (>= _currentphase (`self.FinalPhase`))
    (`self.K2_DestroyActor`))
  (set `self.bCanBeDamaged` true)
  (return true))

(fn `IsPhase`
  (params (Phase :type Integer))
  (returns (Result :type Boolean))
  (if (== (`self.CurrentPhase`) Phase)
    (return true)
    (else
      (return false))))

(fn `SetFireRate`
  (params (`Static Rate` :type "Float (double-precision)") (`Use Random Range` :type Boolean) (Max :type "Float (double-precision)") (Min :type "Float (double-precision)"))
  (if (`self.Shooting`)
    (`self.StopFire`)
    (set `self.Shooting` true))
  (if `Use Random Range`
    (set `self.FireMax` Max)
    (set `self.FireMin` Min)
    (set `self.RandomFireRate` true)
    (else
      (set `self.FireRate` `Static Rate`)
      (set `self.RandomFireRate` false)))
  (if (`self.Shooting`)
    (`self.StartFire`)))

(fn `ShootAnimate`
  (if (`self.ComboAnimFlag`)
    (`self.PlayAnimMontage` (`self.AttackAnim1`) 3.0)
    (set `self.ComboAnimFlag` false)
    (else
      (`self.PlayAnimMontage` (`self.AttackAnim2`) 3.0)
      (set `self.ComboAnimFlag` true))))

(fn `ShootBullet`
  (params (Bullet :type "/Game/Blueprints/BP_ParentEnemyProjectile Class Reference") (Location :type "Vector Structure") (Direction :type "Float (double-precision)") (`Towards Player` :type Boolean :default false))
  (if (`CS330_FinalGameMode.TimeStopped` (`self.My Gamemode`))
    _
    (elif `Towards Player`
      (`|SpawnActorFromClass` Bullet (`KismetMathLibrary.MakeTransform` Location (`KismetMathLibrary.MakeRotator` (.roll (`KismetMathLibrary.FindLookAtRotation` (`self.K2_GetActorLocation`) (`self.K2_GetActorLocation` (`GameplayStatics.GetPlayerCharacter` 0)))) 0.0 (.yaw (`KismetMathLibrary.FindLookAtRotation` (`self.K2_GetActorLocation`) (`self.K2_GetActorLocation` (`GameplayStatics.GetPlayerCharacter` 0)))))) "Undefined" "OverrideRootScale" null null)
      (else
        (`|SpawnActorFromClass` Bullet (`KismetMathLibrary.MakeTransform` Location (`KismetMathLibrary.MakeRotator` (.roll (`self.K2_GetActorRotation`)) 0.0 (+ (.yaw (`self.K2_GetActorRotation`)) Direction))) "Undefined" "OverrideRootScale" null null)))))

(fn `UserConstructionScript`)