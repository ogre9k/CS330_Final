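; BP_MShootOncePerSecond is a bullet emitter that starts firing as soon as play begins.
; BeginPlay calls StartFire, and each FireShot event spawns one BP_E20Circle bullet at Center through ShootBullet.
; The graph holds no timing logic of its own; the name indicates a one-second fire interval.
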(event `self.ReceiveBeginPlay`
  (`parent.ReceiveBeginPlay`)
  (`self.StartFire`))

(event `self.FireShot`
  (`self.Shoot Bullet` "/Game/Blueprints/Bullets/EnemyBullets/BP_E20Circle.BP_E20Circle_C" (`self.Center`)))

(fn `UserConstructionScript`
  (`parent.UserConstructionScript`))