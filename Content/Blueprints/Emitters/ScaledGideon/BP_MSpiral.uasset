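; BP_MSpiral is a projectile emitter in the ScaledGideon set that fires at the player with a pattern chosen by phase.
; It calls the inherited StartFire on BeginPlay, and each FireShot event checks the current phase.
; The first phase shoots a slow homing green orb from Center toward the player.
; The second fires a randomly picked entry from the Bullets array the same way.
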(event `self.ReceiveBeginPlay`
  (`parent.ReceiveBeginPlay`)
  (`self.StartFire`))

(event `self.FireShot`
  (bind _result (`self.IsPhase` 0))
  (if _result
    (`self.Phase1Shoot`)
    (else
      (bind _result_2 (`self.IsPhase` 1))
      (if _result_2
        (`self.Phase2Shoot`)))))

(fn `Phase1Shoot`
  (`self.Shoot Bullet` "/Game/Blueprints/Bullets/EnemyBullets/BP_ESlowHomingGreenOrb.BP_ESlowHomingGreenOrb_C" (`self.Center`) 0.0 true))

(fn `Phase2Shoot`
  (bind _asbp_parent_enemy_projectile (castclass `/Game/Blueprints/BP_ParentEnemyProjectile` (`|GetArrayItem` (`self.Bullets`) (`KismetMathLibrary.RandomInteger` 3))))
  (`self.Shoot Bullet` _asbp_parent_enemy_projectile (`self.Center`) 0.0 true))

(fn `UserConstructionScript`
  (`parent.UserConstructionScript`))