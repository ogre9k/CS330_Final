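; BP_MWall is a bullet emitter that fires walls of enemy projectiles in the first and third phases of a fight.
; It spawns bullets along the Y axis from Center, split into three contiguous segments called columns.
; Phase one fires one random segment with a random bullet type.
; Phase three fires all segments as slow colored orbs, reshuffling colors and briefly pausing after every ten shots.
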(event `self.ReceiveBeginPlay`
  (`parent.ReceiveBeginPlay`)
  (`self.StartFire`))

(event `self.FireShot`
  (bind _result (`self.IsPhase` 0))
  (if _result
    (`self.Phase1Shoot`)
    (else
      (bind _result_2 (`self.IsPhase` 2))
      (if _result_2
        (`self.Phase3Shoot`)
        (if (== (`self.Phase3Counter`) 0)
          (`self.StopFire`)
          (`KismetSystemLibrary.Delay` 1.5)
          (`self.StartFire`))))))

(fn `ColumnSpawn`
  (params (`Loop Index` :type Integer))
  (returns (Location :type "Vector Structure"))
  (return (`KismetMathLibrary.MakeVector` (.x (`self.Center`)) (+ (.y (`self.Center`)) (* 120.0 (`KismetMathLibrary.Conv_IntToDouble` `Loop Index`))) (.z (`self.Center`)))))

(fn `Phase1Shoot`
  (bind _asbp_parent_enemy_projectile (castclass `/Game/Blueprints/BP_ParentEnemyProjectile` (`|GetArrayItem` (`self.Bullets`) (`KismetMathLibrary.RandomInteger` 3))))
  (`self.ShootWallSegment` _asbp_parent_enemy_projectile (`KismetMathLibrary.RandomInteger` 3)))

(fn `Phase3Shoot`
  (bind _phase3random (`self.Phase3Random`))
  ;[1 1 1] Chooses a random wall configuration, rerandomizing every 10 shots
  (if (== (`self.Phase3Counter`) 0)
    (set `self.Phase3Random` (`KismetMathLibrary.RandomInteger` 3))
    (set `self.Phase3Counter` 10))
  (set `self.Phase3Counter` (- (`self.Phase3Counter`) 1))
  (if (== _phase3random 0)
    (`self.ShootWallSegment` "/Game/Blueprints/Bullets/EnemyBullets/BP_ESlowBlueOrb.BP_ESlowBlueOrb_C")
    (`self.ShootWallSegment` "/Game/Blueprints/Bullets/EnemyBullets/BP_ESlowGreenOrb.BP_ESlowGreenOrb_C" 1)
    (`self.ShootWallSegment` "/Game/Blueprints/Bullets/EnemyBullets/BP_ESlowRedOrb.BP_ESlowRedOrb_C" 2)
    (elif (== _phase3random 1)
      (`self.ShootWallSegment` "/Game/Blueprints/Bullets/EnemyBullets/BP_ESlowRedOrb.BP_ESlowRedOrb_C")
      (`self.ShootWallSegment` "/Game/Blueprints/Bullets/EnemyBullets/BP_ESlowBlueOrb.BP_ESlowBlueOrb_C" 1)
      (`self.ShootWallSegment` "/Game/Blueprints/Bullets/EnemyBullets/BP_ESlowGreenOrb.BP_ESlowGreenOrb_C" 2)
      (elif (== _phase3random 2)
        (`self.ShootWallSegment` "/Game/Blueprints/Bullets/EnemyBullets/BP_ESlowGreenOrb.BP_ESlowGreenOrb_C")
        (`self.ShootWallSegment` "/Game/Blueprints/Bullets/EnemyBullets/BP_ESlowRedOrb.BP_ESlowRedOrb_C" 1)
        (`self.ShootWallSegment` "/Game/Blueprints/Bullets/EnemyBullets/BP_ESlowBlueOrb.BP_ESlowBlueOrb_C" 2)))))

(fn `ShootWallSegment`
  (params (Bullet :type "/Game/Blueprints/BP_ParentEnemyProjectile Class Reference") (Column :type Integer))
  (if (== Column 0)
    (for _index (range 1 12)
      (bind _location (`self.ColumnSpawn` _index))
      (`self.Shoot Bullet` Bullet _location))
    (elif (== Column 1)
      (for _index_2 (range 12 23)
        (bind _location_2 (`self.ColumnSpawn` _index_2))
        (`self.Shoot Bullet` Bullet _location_2))
      (elif (== Column 2)
        (for _index_3 (range 23 34)
          (bind _location_3 (`self.ColumnSpawn` _index_3))
          (`self.Shoot Bullet` Bullet _location_3))))))

(fn `UserConstructionScript`
  (`parent.UserConstructionScript`))