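; MyWizardCharacter is a boss-test wizard character Blueprint that pushes its Phase to the bullet or effect emitters in the level.
; BeginPlay and every Tick set Phase to 1, then find all BP_ParentEmitter actors and call UpdatePhase on each.
; An HP-threshold chain for advancing through four phases is present but disconnected, so the phase stays at 1.
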(event `self.ReceiveBeginPlay`
  (set `self.Phase` 1 :!label _label)
  (bind _outactors (`GameplayStatics.GetAllActorsOfClass` "/Game/Blueprints/BP_ParentEmitter.BP_ParentEmitter_C"))
  (for _array_element _outactors
    (`/Game/Blueprints/BP_ParentEmitter.UpdatePhase` _array_element (`self.Phase`))))

(event `self.ReceiveTick`
  (params (DeltaSeconds :type "Float (single-precision)"))
  (goto _label))

(fn `UserConstructionScript`)