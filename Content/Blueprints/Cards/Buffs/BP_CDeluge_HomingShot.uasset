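; Homing water projectile for the Deluge card buff, which seeks the nearest enemy and damages enemies it touches.
; Shortly after spawning, it scans all EnemyCharacters once for the closest and sets that enemy's capsule as the ProjectileMovement homing target.
; Overlapping any EnemyCharacter deals damage and spawns a water-ball hit emitter at the enemy, with no destroy call in the graph.
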(event `self.ReceiveBeginPlay`
  (`KismetSystemLibrary.Delay` 0.2)
  (bind _outactors (`GameplayStatics.GetAllActorsOfClass` "/Script/CS330_Final.EnemyCharacter"))
  (for _array_element _outactors
    (bind _returnvalue (`self.GetDistanceTo` self _array_element))
    (`/Engine/EditorBlueprintResources/StandardMacros.CompareFloat` _returnvalue (`self.SmallestDistance`)
      (:`<`
        (set `self.SmallestDistance` _returnvalue)
        (set `self.ClosestEnemy` _array_element))))
  (set `ProjectileMovementComponent.HomingTargetComponent` (`self.GetComponentByClass` (`self.ClosestEnemy`) "/Script/Engine.CapsuleComponent") (`self.ProjectileMovement`))
  (set `ProjectileMovementComponent.bIsHomingProjectile` true (`self.ProjectileMovement`)))

(event `self.ReceiveActorBeginOverlap`
  (params (OtherActor :type "Actor Object Reference"))
  (bind _asenemy_character (cast `EnemyCharacter` OtherActor))
  (`EnemyCharacter.TakeDamage` _asenemy_character (`self.Damage`) (make `DamageEvent`) (`self.GetInstigatorController`) self)
  (`GameplayStatics.SpawnEmitterAtLocation` "/Game/OurFX/P_ky_waterBallHit.P_ky_waterBallHit" (`self.K2_GetActorLocation` _asenemy_character)))

(fn `UserConstructionScript`)