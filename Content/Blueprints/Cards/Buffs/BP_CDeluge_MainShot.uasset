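; BP_CDeluge_MainShot is the main projectile of a Deluge card buff, damaging enemies with a water-ball hit.
; On spawn it creates two BP_CDeluge_HomingShot actors, offset left and right relative to the player's facing and sharing the player's rotation.
; When it overlaps an EnemyCharacter, it applies its damage through TakeDamage and plays a water hit particle at that enemy's location.
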(event `self.ReceiveBeginPlay`
  (bind _returnvalue (`self.K2_GetActorLocation`))
  (bind _returnvalue_2 (`GameplayStatics.GetPlayerCharacter` 0))
  (bind _returnvalue_3 (`self.K2_GetActorRotation` _returnvalue_2))
  (bind _returnvalue_4 (`KismetMathLibrary.MakeRotFromX` (`self.GetActorForwardVector` _returnvalue_2)))
  (`|SpawnActorFromClass` "/Game/Blueprints/Cards/Buffs/BP_CDeluge_HomingShot.BP_CDeluge_HomingShot_C" (`KismetMathLibrary.MakeTransform` (+ (`KismetMathLibrary.GreaterGreater_VectorRotator` (0.0 90.0 0.0) _returnvalue_4) _returnvalue) _returnvalue_3) "AlwaysSpawn" "OverrideRootScale" null null)
  (`|SpawnActorFromClass` "/Game/Blueprints/Cards/Buffs/BP_CDeluge_HomingShot.BP_CDeluge_HomingShot_C" (`KismetMathLibrary.MakeTransform` (+ _returnvalue (`KismetMathLibrary.GreaterGreater_VectorRotator` (0.0 -90.0 0.0) _returnvalue_4)) _returnvalue_3) "AlwaysSpawn" "OverrideRootScale" null null))

(event `self.ReceiveActorBeginOverlap`
  (params (OtherActor :type "Actor Object Reference"))
  (bind _asenemy_character (cast `EnemyCharacter` OtherActor))
  (`EnemyCharacter.TakeDamage` _asenemy_character (`self.Damage`) (make `DamageEvent`) (`self.GetInstigatorController`) self)
  (`GameplayStatics.SpawnEmitterAtLocation` "/Game/OurFX/P_ky_waterBallHit.P_ky_waterBallHit" (`self.K2_GetActorLocation` _asenemy_character)))

(fn `UserConstructionScript`)