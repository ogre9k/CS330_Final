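; BP_COverheat is the Overheat card buff, which temporarily speeds up the player's firing rate when it begins play.
; It halves BP_PlayerCharacter's FireRate interval for four seconds, then restores it to a hardcoded default rather than the previous value.
; If the player is shooting at either change, it stops and restarts firing so the new rate applies immediately.
; The construction script puts the Overheat artwork on the CardImage brush.
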(event `self.ReceiveBeginPlay`
  (bind _playercharacter (`self.PlayerCharacter`))
  (bind _playercharacter_2 (`self.PlayerCharacter`))
  (bind _playercharacter_3 (`self.PlayerCharacter`))
  (bind _asbp_player_character (cast `/Game/Blueprints/BP_PlayerCharacter` (`GameplayStatics.GetPlayerCharacter` 0)))
  (set `self.PlayerCharacter` _asbp_player_character)
  (if (`PlayerCharacter.Shooting` _playercharacter_2)
    (`PlayerCharacter.OnStopFire` _playercharacter_2)
    (set `PlayerCharacter.FireRate` 0.08 _playercharacter_3)
    (`PlayerCharacter.OnStartFire` _playercharacter_3)
    (else
      (set `PlayerCharacter.FireRate` 0.08 _playercharacter_2)))
  (`KismetSystemLibrary.Delay` 4.0)
  (if (`PlayerCharacter.Shooting` _playercharacter)
    (`PlayerCharacter.OnStopFire` _playercharacter)
    (set `PlayerCharacter.FireRate` 0.16 _playercharacter)
    (`PlayerCharacter.OnStartFire` _playercharacter)
    (else
      (set `PlayerCharacter.FireRate` 0.16 _playercharacter))))

(fn `UserConstructionScript`
  (bind _cardimage (`self.CardImage`))
  (bind (_imagesize _margin _tintcolor _resourceobject _drawas _tiling _mirroring) (break `SlateBrush` (`Image.Brush` _cardimage)))
  (`Image.SetBrush` _cardimage (make `SlateBrush` _imagesize _margin _tintcolor "/Game/Geometry/Images/Card_-_Overheat.Card_-_Overheat" _drawas _tiling _mirroring)))