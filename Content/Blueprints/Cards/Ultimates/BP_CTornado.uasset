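; BP_CTornado is an ultimate card effect that spawns a ring of four tornado helper actors around itself.
; On BeginPlay it calls SpawnTornado for front, back, left and right offsets, then destroys itself.
; Each offset is rotated to player 0's facing and added to the actor's location, and each BP_CTornado_Helper takes the player's rotation and always spawns regardless of collision.
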(event `self.ReceiveBeginPlay`
  (`self.SpawnTornado` (360.0 0.0 0.0))
  (`self.SpawnTornado` (-360.0 0.0 0.0))
  (`self.SpawnTornado` (0.0 360.0 0.0))
  (`self.SpawnTornado` (0.0 -360.0 0.0))
  (`self.K2_DestroyActor`))

(fn `SpawnTornado`
  (params (Offset :type "Vector Structure"))
  (bind _returnvalue (`GameplayStatics.GetPlayerCharacter` 0))
  (`|SpawnActorFromClass` "/Game/Blueprints/Cards/Ultimates/BP_CTornado_Helper.BP_CTornado_Helper_C" (`KismetMathLibrary.MakeTransform` (+ (`self.K2_GetActorLocation`) (`KismetMathLibrary.GreaterGreater_VectorRotator` (`local.Offset`) (`KismetMathLibrary.MakeRotFromX` (`self.GetActorForwardVector` _returnvalue)))) (`self.K2_GetActorRotation` _returnvalue)) "AlwaysSpawn" "OverrideRootScale" null null))

(fn `UserConstructionScript`)