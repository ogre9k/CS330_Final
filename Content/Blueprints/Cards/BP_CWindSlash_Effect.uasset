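; BP_CWindSlash_Effect is the effect actor for a Wind Slash card that sweeps through an arc and damages enemies it touches.
; On BeginPlay it turns back 90 degrees in yaw, then a timeline lerps its rotation through 180 degrees to swing across the front.
; Any EnemyCharacter that begins overlapping the actor takes its Damage value, credited to the instigator's controller.
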(event `self.ReceiveBeginPlay`
  (bind _returnvalue (`self.K2_GetActorRotation`))
  (`self.K2_SetActorRotation` (`KismetMathLibrary.MakeRotator` (.roll (`self.K2_GetActorRotation`)) (.pitch (`self.K2_GetActorRotation`)) (+ (.yaw (`self.K2_GetActorRotation`)) -90.0)))
  (set `self.InitialRotation` _returnvalue)
  (set `self.Target Rotation` (`KismetMathLibrary.MakeRotator` (.roll _returnvalue) (.pitch _returnvalue) (+ (.yaw _returnvalue) 180.0)))
  (bind (_direction _newtrack_0) (`Timeline|Timeline_0`)
    (:`Update`
      (`self.K2_SetActorRotation` (`KismetMathLibrary.RLerp` (`self.InitialRotation`) (`self.Target Rotation`) _newtrack_0)))))

(event `self.ReceiveActorBeginOverlap`
  (params (OtherActor :type "Actor Object Reference"))
  (bind _asenemy_character (cast `EnemyCharacter` OtherActor))
  (`EnemyCharacter.TakeDamage` _asenemy_character (`self.Damage`) (make `DamageEvent`) (`self.GetInstigatorController`) self))

(event `self.ReceiveTick`
  (params (DeltaSeconds :type "Float (single-precision)")))

(fn `UserConstructionScript`)