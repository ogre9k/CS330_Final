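; BP_CHitEffect is a card hit effect actor: a short-lived explosion hitbox meant to damage enemies it touches.
; Begin overlap applies Damage to EnemyCharacter actors, gated by the Active flag and credited to the instigator's controller.
; A 0.1-second delay after BeginPlay sets Active to true and immediately disables the Sphere's collision to close the damage window.
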(event `self.ReceiveBeginPlay`
  ;[1 1 1] 0.1 seconds after spawning, the explosion can't hurt enemies anymore
  (`KismetSystemLibrary.Delay` 0.1)
  (set `self.Active` true)
  (`PrimitiveComponent.SetCollisionEnabled` (`self.Sphere`) "NoCollision"))

(event `self.ReceiveActorBeginOverlap`
  (params (OtherActor :type "Actor Object Reference"))
  (if (`self.Active`)
    (bind _asenemy_character (cast `EnemyCharacter` OtherActor))
    (`EnemyCharacter.TakeDamage` _asenemy_character (`self.Damage`) (make `DamageEvent`) (`self.GetInstigatorController`) self)))

(fn `UserConstructionScript`)