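; Boomerang card attack projectile that damages enemies it overlaps as it homes back to the player.
; On BeginPlay it sets the player's capsule as the ProjectileMovement homing target, then enables homing after a brief delay to create the return arc.
; Each enemy overlap applies damage credited to the instigator and spawns a wind-ball hit particle at that enemy.
; The overlap logic never destroys the projectile, so it can hit several enemies.
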(event `self.ReceiveBeginPlay`
  (set `ProjectileMovementComponent.HomingTargetComponent` (`self.GetComponentByClass` (`GameplayStatics.GetPlayerCharacter` 0) "/Script/Engine.CapsuleComponent") (`self.ProjectileMovement`))
  (`KismetSystemLibrary.Delay` 0.1)
  (set `ProjectileMovementComponent.bIsHomingProjectile` true (`self.ProjectileMovement`)))

(event `self.ReceiveActorBeginOverlap`
  (params (OtherActor :type "Actor Object Reference"))
  (bind _asenemy_character (cast `EnemyCharacter` OtherActor))
  (`EnemyCharacter.TakeDamage` _asenemy_character (`self.Damage`) (make `DamageEvent`) (`self.GetInstigatorController`) self)
  (`GameplayStatics.SpawnEmitterAtLocation` "/Game/OurFX/P_ky_windBallHit.P_ky_windBallHit" (`self.K2_GetActorLocation` _asenemy_character)))

(fn `UserConstructionScript`)