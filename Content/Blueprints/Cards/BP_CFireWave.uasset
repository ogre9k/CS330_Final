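; BP_CFireWave is a fire wave actor, filed under Cards, that fires a fan of BP_CFireWave_Helper actors when it begins play.
; BeginPlay loops over ShootFire, stepping a yaw offset by a fixed increment from a negative starting angle.
; ShootFire spawns each helper at the actor's location with that offset added to its yaw, always spawning regardless of collision.
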(event `self.ReceiveBeginPlay`
  (set `self.Offset` -8.0)
  (for _ (range 11)
    (`self.ShootFire` (`self.Offset`))
    (set `self.Offset` (+ (`self.Offset`) 2.0))))

(fn `ShootFire`
  (params (`Yaw Offset` :type "Float (double-precision)"))
  (`|SpawnActorFromClass` "/Game/Blueprints/Cards/BP_CFireWave_Helper.BP_CFireWave_Helper_C" (`KismetMathLibrary.MakeTransform` (`self.K2_GetActorLocation`) (`KismetMathLibrary.MakeRotator` (.roll (`self.K2_GetActorRotation`)) (.pitch (`self.K2_GetActorRotation`)) (+ (.yaw (`self.K2_GetActorRotation`)) `Yaw Offset`))) "AlwaysSpawn" "OverrideRootScale" null null))

(fn `UserConstructionScript`)