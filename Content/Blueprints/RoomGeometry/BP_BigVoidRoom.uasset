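; BP_BigVoidRoom is a room geometry Blueprint with two gates and a door trigger.
; The OpenDoor event destroys the Gate and the DoorTrigger through OpenGate when it reports all enemies killed.
; A player character overlapping the DoorTrigger destroys Gate2 and the trigger itself.
; Both paths remove the same trigger, so opening Gate first leaves Gate2 without its overlap opener.
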(event `self.OpenDoor`
  (params (AllEnemiesKilled :type Boolean))
  (if AllEnemiesKilled
    (`self.OpenGate`)))

(event `self.DoorTrigger.OnComponentBeginOverlap`
  (params (OverlappedComponent :type "PrimitiveComponent Object Reference") (OtherActor :type "Actor Object Reference") (OtherComp :type "PrimitiveComponent Object Reference") (OtherBodyIndex :type Integer) (bFromSweep :type Boolean) (SweepResult :type "HitResult Structure (by ref)"))
  (cast `/Game/Blueprints/BP_PlayerCharacter` OtherActor)
  (`ActorComponent.K2_DestroyComponent` (`self.Gate2`))
  (`ActorComponent.K2_DestroyComponent` (`self.DoorTrigger`)))

(fn `OpenGate`
  (`ActorComponent.K2_DestroyComponent` (`self.Gate`))
  (`ActorComponent.K2_DestroyComponent` (`self.DoorTrigger`)))

(fn `UserConstructionScript`)