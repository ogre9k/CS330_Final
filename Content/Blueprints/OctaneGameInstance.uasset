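; Game instance that holds the player's card deck layout in GlobalDeckData, indexed by catalog card.
; ModifyGlobalDeck waits a second, then initializes the array if its first entry is -1, otherwise rebuilds the player's decks from it.
; Initialization scans Hand, Deck and NotInPlay, mapping card classes to indices through counting if-chains.
; Rebuilding clears MyDeck and passes each entry and its index to GetFromCatalog.
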(event `ModifyGlobalDeck`
  (`KismetSystemLibrary.Delay` 1.0)
  (if (== (`|GetArrayItem` (`self.GlobalDeckData`)) -1)
    (`self.InitializeGlobalDeck`)
    (else
      (`self.UpdateGlobalDeck`))))

(fn `InitializeGlobalDeck`
  (bind _settingindex (`self.SettingIndex`))
  (bind _settingindex_2 (`self.SettingIndex`))
  (bind _settingindex_3 (`self.SettingIndex`))
  ;[1 1 1] Record what's in the hand.
  (bind _asoctane_game_instance (cast `/Game/Blueprints/OctaneGameInstance` (`GameplayStatics.GetGameInstance`)))
  (bind _asbp_player_character (cast `/Game/Blueprints/BP_PlayerCharacter` (`GameplayStatics.GetPlayerCharacter` 0)))
  (for _array_element (`DeckHandler._hand` (`PlayerCharacter.MyDeck` _asbp_player_character))
    (if (== _array_element "/Game/Blueprints/Cards/Cantrips/BP_CEmber.BP_CEmber_C")
      (bind _globaldeckdata (`/Game/Blueprints/OctaneGameInstance.GlobalDeckData` _asoctane_game_instance))
      (`KismetArrayLibrary.Array_Set` _globaldeckdata _settingindex_3 :!label _label)
      (set `self.SettingIndex` 0)
      (else
        (`/Engine/EditorBlueprintResources/StandardMacros.IncrementInt` _settingindex_3
          (:`  `
            (if (== _array_element "/Game/Blueprints/Cards/Cantrips/BP_CDroplet.BP_CDroplet_C")
              (goto _label)
              (else
                (`/Engine/EditorBlueprintResources/StandardMacros.IncrementInt` _settingindex_3
                  (:`  `
                    (if (== _array_element "/Game/Blueprints/Cards/Cantrips/BP_CBreeze.BP_CBreeze_C")
                      (goto _label)
                      (else
                        (`/Engine/EditorBlueprintResources/StandardMacros.IncrementInt` _settingindex_3
                          (:`  `
                            (if (== _array_element "/Game/Blueprints/Cards/Attacks/BP_CFireball.BP_CFireball_C")
                              (goto _label)
                              (else
                                (`/Engine/EditorBlueprintResources/StandardMacros.IncrementInt` _settingindex_3
                                  (:`  `
                                    (if (== _array_element "/Game/Blueprints/Cards/Attacks/BP_CBurst.BP_CBurst_C")
                                      (goto _label)
                                      (else
                                        (`/Engine/EditorBlueprintResources/StandardMacros.IncrementInt` _settingindex_3
                                          (:`  `
                                            (if (== _array_element "/Game/Blueprints/Cards/Attacks/BP_CBoomerang.BP_CBoomerang_C")
                                              (goto _label)
                                              (else
                                                (`/Engine/EditorBlueprintResources/StandardMacros.IncrementInt` _settingindex_3
                                                  (:`  `
                                                    (if (== _array_element "/Game/Blueprints/Cards/Buffs/BP_COverheat.BP_COverheat_C")
                                                      (goto _label)
                                                      (else
                                                        (`/Engine/EditorBlueprintResources/StandardMacros.IncrementInt` _settingindex_3
                                                          (:`  `
                                                            (if (== _array_element "/Game/Blueprints/Cards/Buffs/BP_CDeluge.BP_CDeluge_C")
                                                              (goto _label)
                                                              (else
                                                                (`/Engine/EditorBlueprintResources/StandardMacros.IncrementInt` _settingindex_3
                                                                  (:`  `
                                                                    (if (== _array_element "/Game/Blueprints/Cards/Buffs/BP_CBlitz.BP_CBlitz_C")
                                                                      (goto _label)
                                                                      (else
                                                                        (`/Engine/EditorBlueprintResources/StandardMacros.IncrementInt` _settingindex_3
                                                                          (:`  `
                                                                            (if (== _array_element "/Game/Blueprints/Cards/Ultimates/BP_CInferno.BP_CInferno_C")
                                                                              (goto _label)
                                                                              (else
                                                                                (`/Engine/EditorBlueprintResources/StandardMacros.IncrementInt` _settingindex_3
                                                                                  (:`  `
                                                                                    (if (== _array_element "/Game/Blueprints/Cards/Ultimates/BP_CFreeze.BP_CFreeze_C")
                                                                                      (goto _label)
                                                                                      (else
                                                                                        (`/Engine/EditorBlueprintResources/StandardMacros.IncrementInt` _settingindex_3
                                                                                          (:`  `
                                                                                            (if (== _array_element "/Game/Blueprints/Cards/Ultimates/BP_CTornado.BP_CTornado_C")
                                                                                              (goto _label)))))))))))))))))))))))))))))))))))))))))))))))
  ;[1 1 1] Record what's in the deck.
  (cast `/Game/Blueprints/OctaneGameInstance` (`GameplayStatics.GetGameInstance`))
  (bind _asbp_player_character_2 (cast `/Game/Blueprints/BP_PlayerCharacter` (`GameplayStatics.GetPlayerCharacter` 0)))
  (for _array_element_2 (`DeckHandler._deck` (`PlayerCharacter.MyDeck` _asbp_player_character_2))
    (if (== _array_element_2 "/Game/Blueprints/Cards/Cantrips/BP_CEmber.BP_CEmber_C")
      (`KismetArrayLibrary.Array_Set` _globaldeckdata _settingindex :!label _label_2)
      (set `self.SettingIndex` 0)
      (else
        (`/Engine/EditorBlueprintResources/StandardMacros.IncrementInt` _settingindex
          (:`  `
            (if (== _array_element_2 "/Game/Blueprints/Cards/Cantrips/BP_CDroplet.BP_CDroplet_C")
              (goto _label_2)
              (else
                (`/Engine/EditorBlueprintResources/StandardMacros.IncrementInt` _settingindex
                  (:`  `
                    (if (== _array_element_2 "/Game/Blueprints/Cards/Cantrips/BP_CBreeze.BP_CBreeze_C")
                      (goto _label_2)
                      (else
                        (`/Engine/EditorBlueprintResources/StandardMacros.IncrementInt` _settingindex
                          (:`  `
                            (if (== _array_element_2 "/Game/Blueprints/Cards/Attacks/BP_CFireball.BP_CFireball_C")
                              (goto _label_2)
                              (else
                                (`/Engine/EditorBlueprintResources/StandardMacros.IncrementInt` _settingindex
                                  (:`  `
                                    (if (== _array_element_2 "/Game/Blueprints/Cards/Attacks/BP_CBurst.BP_CBurst_C")
                                      (goto _label_2)
                                      (else
                                        (`/Engine/EditorBlueprintResources/StandardMacros.IncrementInt` _settingindex
                                          (:`  `
                                            (if (== _array_element_2 "/Game/Blueprints/Cards/Attacks/BP_CBoomerang.BP_CBoomerang_C")
                                              (goto _label_2)
                                              (else
                                                (`/Engine/EditorBlueprintResources/StandardMacros.IncrementInt` _settingindex
                                                  (:`  `
                                                    (if (== _array_element_2 "/Game/Blueprints/Cards/Buffs/BP_COverheat.BP_COverheat_C")
                                                      (goto _label_2)
                                                      (else
                                                        (`/Engine/EditorBlueprintResources/StandardMacros.IncrementInt` _settingindex
                                                          (:`  `
                                                            (if (== _array_element_2 "/Game/Blueprints/Cards/Buffs/BP_CDeluge.BP_CDeluge_C")
                                                              (goto _label_2)
                                                              (else
                                                                (`/Engine/EditorBlueprintResources/StandardMacros.IncrementInt` _settingindex
                                                                  (:`  `
                                                                    (if (== _array_element_2 "/Game/Blueprints/Cards/Buffs/BP_CBlitz.BP_CBlitz_C")
                                                                      (goto _label_2)
                                                                      (else
                                                                        (`/Engine/EditorBlueprintResources/StandardMacros.IncrementInt` _settingindex
                                                                          (:`  `
                                                                            (if (== _array_element_2 "/Game/Blueprints/Cards/Ultimates/BP_CInferno.BP_CInferno_C")
                                                                              (goto _label_2)
                                                                              (else
                                                                                (`/Engine/EditorBlueprintResources/StandardMacros.IncrementInt` _settingindex
                                                                                  (:`  `
                                                                                    (if (== _array_element_2 "/Game/Blueprints/Cards/Ultimates/BP_CFreeze.BP_CFreeze_C")
                                                                                      (goto _label_2)
                                                                                      (else
                                                                                        (`/Engine/EditorBlueprintResources/StandardMacros.IncrementInt` _settingindex
                                                                                          (:`  `
                                                                                            (if (== _array_element_2 "/Game/Blueprints/Cards/Ultimates/BP_CTornado.BP_CTornado_C")
                                                                                              (goto _label_2)))))))))))))))))))))))))))))))))))))))))))))))
  ;[1 1 1] Record what's in notInPlay.
  (cast `/Game/Blueprints/OctaneGameInstance` (`GameplayStatics.GetGameInstance`))
  (bind _asbp_player_character_3 (cast `/Game/Blueprints/BP_PlayerCharacter` (`GameplayStatics.GetPlayerCharacter` 0)))
  (for _array_element_3 (`DeckHandler._notInPlay` (`PlayerCharacter.MyDeck` _asbp_player_character_3))
    (if (== _array_element_3 "/Game/Blueprints/Cards/Cantrips/BP_CEmber.BP_CEmber_C")
      (`KismetArrayLibrary.Array_Set` _globaldeckdata _settingindex_2 :!label _label_3)
      (set `self.SettingIndex` 0)
      (else
        (`/Engine/EditorBlueprintResources/StandardMacros.IncrementInt` _settingindex_2
          (:`  `
            (if (== _array_element_3 "/Game/Blueprints/Cards/Cantrips/BP_CDroplet.BP_CDroplet_C")
              (goto _label_3)
              (else
                (`/Engine/EditorBlueprintResources/StandardMacros.IncrementInt` _settingindex_2
                  (:`  `
                    (if (== _array_element_3 "/Game/Blueprints/Cards/Cantrips/BP_CBreeze.BP_CBreeze_C")
                      (goto _label_3)
                      (else
                        (`/Engine/EditorBlueprintResources/StandardMacros.IncrementInt` _settingindex_2
                          (:`  `
                            (if (== _array_element_3 "/Game/Blueprints/Cards/Attacks/BP_CFireball.BP_CFireball_C")
                              (goto _label_3)
                              (else
                                (`/Engine/EditorBlueprintResources/StandardMacros.IncrementInt` _settingindex_2
                                  (:`  `
                                    (if (== _array_element_3 "/Game/Blueprints/Cards/Attacks/BP_CBurst.BP_CBurst_C")
                                      (goto _label_3)
                                      (else
                                        (`/Engine/EditorBlueprintResources/StandardMacros.IncrementInt` _settingindex_2
                                          (:`  `
                                            (if (== _array_element_3 "/Game/Blueprints/Cards/Attacks/BP_CBoomerang.BP_CBoomerang_C")
                                              (goto _label_3)
                                              (else
                                                (`/Engine/EditorBlueprintResources/StandardMacros.IncrementInt` _settingindex_2
                                                  (:`  `
                                                    (if (== _array_element_3 "/Game/Blueprints/Cards/Buffs/BP_COverheat.BP_COverheat_C")
                                                      (goto _label_3)
                                                      (else
                                                        (`/Engine/EditorBlueprintResources/StandardMacros.IncrementInt` _settingindex_2
                                                          (:`  `
                                                            (if (== _array_element_3 "/Game/Blueprints/Cards/Buffs/BP_CDeluge.BP_CDeluge_C")
                                                              (goto _label_3)
                                                              (else
                                                                (`/Engine/EditorBlueprintResources/StandardMacros.IncrementInt` _settingindex_2
                                                                  (:`  `
                                                                    (if (== _array_element_3 "/Game/Blueprints/Cards/Buffs/BP_CBlitz.BP_CBlitz_C")
                                                                      (goto _label_3)
                                                                      (else
                                                                        (`/Engine/EditorBlueprintResources/StandardMacros.IncrementInt` _settingindex_2
                                                                          (:`  `
                                                                            (if (== _array_element_3 "/Game/Blueprints/Cards/Ultimates/BP_CInferno.BP_CInferno_C")
                                                                              (goto _label_3)
                                                                              (else
                                                                                (`/Engine/EditorBlueprintResources/StandardMacros.IncrementInt` _settingindex_2
                                                                                  (:`  `
                                                                                    (if (== _array_element_3 "/Game/Blueprints/Cards/Ultimates/BP_CFreeze.BP_CFreeze_C")
                                                                                      (goto _label_3)
                                                                                      (else
                                                                                        (`/Engine/EditorBlueprintResources/StandardMacros.IncrementInt` _settingindex_2
                                                                                          (:`  `
                                                                                            (if (== _array_element_3 "/Game/Blueprints/Cards/Ultimates/BP_CTornado.BP_CTornado_C")
                                                                                              (goto _label_3))))))))))))))))))))))))))))))))))))))))))))))))

(fn `UpdateGlobalDeck`
  ;[1 1 1] Clear the decks before repopulating them.
  (bind _asoctane_game_instance (cast `/Game/Blueprints/OctaneGameInstance` (`GameplayStatics.GetGameInstance`)))
  (bind _asbp_player_character (cast `/Game/Blueprints/BP_PlayerCharacter` (`GameplayStatics.GetPlayerCharacter` 0)))
  (bind _mydeck (`PlayerCharacter.MyDeck` _asbp_player_character))
  (`DeckHandler.ClearDecks` _mydeck)
  ;[1 1 1] Repopulate the decks.
  (for (_array_element _array_index) (`/Game/Blueprints/OctaneGameInstance.GlobalDeckData` _asoctane_game_instance)
    (`DeckHandler.GetFromCatalog` _mydeck _array_element _array_index)))