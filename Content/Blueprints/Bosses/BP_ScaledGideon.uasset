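; Gideon boss, a child Blueprint that fires aimed red orbs and seven-way blue orb fans according to its current phase.
; A looping timer spawns spirals on the player during phases two and four, unless time is stopped.
; Phase changes discard the player's hand and adjust fire rate.
; Phase five plays death, then updates the deck and opens Final3, a sequence EndPlay also enters at its delay.
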(event `self.ReceiveBeginPlay`
  (bind _ascs330_final_game_mode (cast `CS330_FinalGameMode` (`GameplayStatics.GetGameMode`)))
  (set `self.My Gamemode` _ascs330_final_game_mode)
  (`KismetSystemLibrary.K2_SetTimer` self "SpawnSpiral" 3.0 true)
  (`self.UpdateOffsets`)
  (`self.StartFire`))

(event `self.ReceiveActorBeginOverlap`
  (params (OtherActor :type "Actor Object Reference"))
  (`parent.ReceiveActorBeginOverlap` OtherActor))

(event `self.ReceiveTick`
  (params (DeltaSeconds :type "Float (single-precision)"))
  (`parent.ReceiveTick` DeltaSeconds)
  (`self.UpdateFacing`))

(event `self.FireShot`
  (bind _result (`self.IsPhase` 1))
  (if _result
    (if (== (`self.Shot Counter`) 10)
      (`self.SpreadShot`)
      (set `self.Shot Counter` 0)
      (else
        (`self.SingleShot`)
        (set `self.Shot Counter` (+ (`self.Shot Counter`) 1))))
    (else
      (bind _result_2 (`self.IsPhase` 3))
      (if _result_2
        (`self.SingleShot`)
        (else
          (bind _result_3 (`self.IsPhase` 4))
          (if _result_3
            (`self.SpreadShot`)))))))

(event `self.ChangePhase`
  (`self.HandleNewPhase`)
  (`self.GideonHandlePhase`)
  (bind _outactors (`GameplayStatics.GetAllActorsOfClass` "/Script/CS330_Final.DeckHandler"))
  (for _array_element _outactors
    (`DeckHandler.DiscardHand` _array_element)
    (bind _result (`self.IsPhase` 5))
    (if _result
      (bind _returnvalue (`self.PlayAnimMontage` "/Game/Blueprints/Death_Anim.Death_Anim"))
      (`KismetSystemLibrary.Delay` _returnvalue :!label _label)
      (bind _asoctane_game_instance (cast `/Game/Blueprints/OctaneGameInstance` (`GameplayStatics.GetGameInstance`)))
      (bind _asbp_player_character (cast `/Game/Blueprints/BP_PlayerCharacter` (`GameplayStatics.GetPlayerCharacter` 0)))
      (`DeckHandler.AddToDeck` (`PlayerCharacter.MyDeck` _asbp_player_character))
      (`/Game/Blueprints/OctaneGameInstance.UpdateGlobalDeck` _asoctane_game_instance)
      (`GameplayStatics.OpenLevel` "Final3"))))

(event `self.ReceiveEndPlay`
  (params (EndPlayReason :type "EEndPlayReason Enum" :default "Destroyed"))
  (goto _label))

(fn `GideonHandlePhase`
  (returns (`N/A` :type Boolean))
  (`|SpawnActorFromClass` "/Game/Blueprints/Cards/BP_CHitEffect.BP_CHitEffect_C" (`KismetMathLibrary.Conv_VectorToTransform` (`self.Center`)) "Undefined" "OverrideRootScale" null null)
  (bind _result (`self.IsPhase` 4))
  (if _result
    (`self.SetFireRate` 1.5)
    (else
      (bind _result_2 (`self.IsPhase` 3))
      (if _result_2
        (`self.SetFireRate` 3.0)
        (return false)))))

(fn `SingleShot`
  (`self.ShootAnimate`)
  (`self.ShootBullet` "/Game/Blueprints/Bullets/EnemyBullets/BP_ERedOrb.BP_ERedOrb_C" (`KismetMathLibrary.MakeVector` (.x (`self.Front`)) (.y (`self.Front`)) (- (.z (`self.Front`)) 250.0)) 0.0 true))

(fn `SpawnSpiral`
  (if (or (== (`self.CurrentPhase`) 2) (== (`self.CurrentPhase`) 4))
    (if (not (`CS330_FinalGameMode.TimeStopped` (`self.My Gamemode`)))
      (`|SpawnActorFromClass` "/Game/Blueprints/Emitters/ScaledGideon/BP_MSpiral.BP_MSpiral_C" (`KismetMathLibrary.MakeTransform` (`self.K2_GetActorLocation` (`GameplayStatics.GetPlayerCharacter` 0)) (`self.K2_GetActorRotation`)) "AlwaysSpawn" "OverrideRootScale" null null))))

(fn `SpreadShot`
  (`self.ShootAnimate`)
  (for _index (range 7)
    (`self.ShootBullet` "/Game/Blueprints/Bullets/EnemyBullets/BP_EBlueOrb.BP_EBlueOrb_C" (`KismetMathLibrary.MakeVector` (.x (`self.Front`)) (.y (`self.Front`)) (- (.z (`self.Front`)) 250.0)) (+ (* _index 15.0) -45.0))))

(fn `UserConstructionScript`
  (`parent.UserConstructionScript`))