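; Parent enemy projectile Blueprint that responds to the game's time-stop state and can spawn further bullets.
; On BeginPlay it caches the game mode and initial velocity, then calls UpdateOffsets.
; StopTime zeroes the movement velocity while time is stopped and otherwise restores the cached velocity.
; ShootBullet spawns a given class only while time runs, flattening pitch and aiming at the player or at a yaw offset from its own rotation.
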(event `self.ReceiveBeginPlay`
  ;[1 1 1] Handling for timestop
  (bind _ascs330_final_game_mode (cast `CS330_FinalGameMode` (`GameplayStatics.GetGameMode`)))
  (set `self.MyGameMode` _ascs330_final_game_mode)
  (set `self.InitialVelocity` (`MovementComponent.Velocity` (`self.ProjectileMovement`)))
  (`self.UpdateOffsets`))

(event `StopTime`
  ;[1 1 1] Handling for timestop
  (if (`CS330_FinalGameMode.TimeStopped` (`self.MyGameMode`))
    (set `MovementComponent.Velocity` (0.0 0.0 0.0) (`self.ProjectileMovement`))
    (else
      (set `MovementComponent.Velocity` (`self.InitialVelocity`) (`self.ProjectileMovement`)))))

(fn `Shoot Bullet`
  (params (Bullet :type "EnemyProjectile Class Reference") (Location :type "Vector Structure") (Direction :type "Float (double-precision)") (`Towards Player` :type Boolean))
  (if (`CS330_FinalGameMode.TimeStopped` (`self.MyGameMode`))
    _
    (elif `Towards Player`
      (`|SpawnActorFromClass` Bullet (`KismetMathLibrary.MakeTransform` Location (`KismetMathLibrary.MakeRotator` (.roll (`KismetMathLibrary.FindLookAtRotation` (`self.K2_GetActorLocation`) (`self.K2_GetActorLocation` (`GameplayStatics.GetPlayerCharacter` 0)))) 0.0 (.yaw (`KismetMathLibrary.FindLookAtRotation` (`self.K2_GetActorLocation`) (`self.K2_GetActorLocation` (`GameplayStatics.GetPlayerCharacter` 0)))))) "Undefined" "OverrideRootScale" null null)
      (else
        (`|SpawnActorFromClass` Bullet (`KismetMathLibrary.MakeTransform` Location (`KismetMathLibrary.MakeRotator` (.roll (`self.K2_GetActorRotation`)) 0.0 (+ (.yaw (`self.K2_GetActorRotation`)) Direction))) "Undefined" "OverrideRootScale" null null)))))

(fn `UserConstructionScript`)