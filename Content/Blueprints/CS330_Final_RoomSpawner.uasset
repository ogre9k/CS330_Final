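; Room spawner Blueprint that chains Room0 actors together when play begins.
; BeginPlay calls AddRoom in a short loop, spawning each room at the NextRoomSpawn transform.
; Each new room's GetAttachTransform result becomes the next spawn point, so rooms line up end to end.
; AddHallway spawns a Hallway at NextHallwaySpawn, but nothing here calls it or updates that transform.
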(event `self.ReceiveBeginPlay`
  (for _ (range 2)
    (`self.AddRoom`)))

(fn `AddHallway`
  (`|SpawnActorFromClass` "/Game/Blueprints/Hallway.Hallway_C" (`self.NextHallwaySpawn`) "Undefined" "OverrideRootScale" null null))

(fn `AddRoom`
  (bind _returnvalue (`|SpawnActorFromClass` "/Game/Blueprints/Room0.Room0_C" (`self.NextRoomSpawn`) "Undefined" "OverrideRootScale" null null))
  (bind _asroom_0 (cast `/Game/Blueprints/Room0` _returnvalue))
  (bind _attachtransform (`/Game/Blueprints/Room0.GetAttachTransform` _asroom_0))
  (set `self.NextRoomSpawn` _attachtransform))

(fn `UserConstructionScript`)